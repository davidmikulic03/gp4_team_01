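; BP_InteractableElectricalBox is an interactable electrical box that makes noise when the player uses it.
; On interact it gets the noise system from MainGameMode and registers a noise event at its location using the InteractableButton noise data asset.
; Interactable state toggles an outline overlay material on the ElectricalBox mesh as a highlight.
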(event `self.ReceiveBeginPlay`)

(event `self.OnInteract`
  (params (Caller :type "Actor Object Reference"))
  (bind _asmain_game_mode (cast `MainGameMode` (`GameplayStatics.GetGameMode`)))
  (bind _returnvalue (`MainGameMode.GetNoiseSystemRef` _asmain_game_mode))
  (`NoiseSystem.RegisterNoiseEvent` _returnvalue "/Game/DataAssets/Noise/Assets/InteractableButton.InteractableButton" (`self.K2_GetActorLocation`)))

(event `self.OnInteractable`
  (`MeshComponent.SetOverlayMaterial` (`self.ElectricalBox`) "/Game/MaterialLibrary/Outline_M.Outline_M"))

(event `self.OnNotInteractable`
  (`MeshComponent.SetOverlayMaterial` (`self.ElectricalBox`) null))

(fn `UserConstructionScript`)