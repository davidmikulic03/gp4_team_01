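; Interactable platform that rotates from its starting world rotation toward a target rotation, with FMOD sound.
; BeginPlay caches the initial rotation, and while IsOpening is true Tick lerps the root toward Rotation by the fade timer ratio, neither flag nor timer being updated here.
; Interacting starts the active sound at the platform and stores its instance; un-interacting stops it and plays a stop sound.
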(event `self.ReceiveBeginPlay`
  (set `self.InitialRotation` (`SceneComponent.K2_GetComponentRotation` (`self.RootComponent`))))

(event `self.ReceiveTick`
  (params (DeltaSeconds :type "Float (single-precision)"))
  (if (`self.bIsOpening`)
    (`SceneComponent.K2_SetWorldRotation` (`self.RootComponent`) (`KismetMathLibrary.RLerp` (`self.InitialRotation`) (`self.Rotation`) (/ (`self.CurrentFadeTimer`) (`self.TimeToFadeOpen`))) false false)))

(event `self.OnInteractEvent`
  (bind _returnvalue (`FMODBlueprintStatics.PlayEventAtLocation` "/Game/FMOD/Events/Platform_Active.Platform_Active" (`KismetMathLibrary.Conv_VectorToTransform` (`SceneComponent.K2_GetComponentLocation` (`self.RootComponent`)))))
  (set `self.Sound` _returnvalue))

(event `self.OnUnInteractEvent`
  (`FMODBlueprintStatics.EventInstanceStop` (`self.Sound`))
  (`FMODBlueprintStatics.PlayEventAtLocation` "/Game/FMOD/Events/Platform_Stop.Platform_Stop" (`KismetMathLibrary.Conv_VectorToTransform` (`SceneComponent.K2_GetComponentLocation` (`self.RootComponent`)))))

(fn `UserConstructionScript`)