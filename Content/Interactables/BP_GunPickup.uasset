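; Interactable gun pickup that activates the player's gun and removes itself from the world.
; On interact, it calls ActivateGun on the calling PlayerCharacter, shows its pickup text on the WB_PlayerHUD widget and destroys the actor.
; An overlay outline material on the static mesh highlights the pickup while it is interactable and is cleared when it is not.
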(event `self.OnInteract`
  (params (Caller :type "Actor Object Reference"))
  (bind _asplayer_character (cast `PlayerCharacter` Caller)
    (:`then`
      (`PlayerCharacter.ActivateGun` _asplayer_character))
    (:`CastFailed`
      _))
  (`self.K2_DestroyActor`)
  (bind _foundwidgets (`WidgetBlueprintLibrary.GetAllWidgetsOfClass` "/Game/UI/WB_PlayerHUD.WB_PlayerHUD_C"))
  (`/Game/UI/WB_PlayerHUD.Show Pickup Text` (`|GetArrayItem` _foundwidgets) (`self.TextOnInteract`))
  (`self.K2_DestroyActor`))

(event `self.OnInteractable`
  (`MeshComponent.SetOverlayMaterial` (`self.StaticMesh`) "/Game/MaterialLibrary/Outline_M.Outline_M"))

(event `self.OnNotInteractable`
  (`MeshComponent.SetOverlayMaterial` (`self.StaticMesh`) null))

(fn `UserConstructionScript`)