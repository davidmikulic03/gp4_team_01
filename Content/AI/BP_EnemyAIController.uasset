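; Enemy AI controller that runs the base enemy behavior tree and feeds it perception data.
; On BeginPlay it starts BT_BaseEnemy.
; Perception updates from sight store the sensed actor as PlayerActor on the Blackboard, while any other sense writes the stimulus location as TargetLocation.
; The sight branch does not check whether sensing succeeded or whether the actor is the player.
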(event `self.ReceiveBeginPlay`
  (`self.RunBehaviorTree` "/Game/AI/BT_BaseEnemy.BT_BaseEnemy"))

(event `self.AIPerception.OnTargetPerceptionUpdated`
  (params (Actor :type "Actor Object Reference") (Stimulus :type "AIStimulus Structure"))
  (bind _returnvalue (`AIPerceptionSystem.GetSenseClassForStimulus` Stimulus))
  (if (== _returnvalue "/Script/AIModule.AISense_Sight")
    (`BlackboardComponent.SetValueAsObject` (`self.Blackboard`) "PlayerActor" Actor)
    (else
      (`BlackboardComponent.SetValueAsVector` (`self.Blackboard`) "TargetLocation" (`.StimulusLocation` (break `AIStimulus` Stimulus))))))

(fn `UserConstructionScript`)