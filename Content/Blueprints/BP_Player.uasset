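; Player Blueprint that drives a crouch vignette and forwards inventory changes to the HUD.
; BeginPlay adds a dynamic vignette material to the camera's post-process blendables, and crouch start and end toggle its SecondaryOpacity parameter.
; Inventory updates refresh the rock and smoke bomb counts through PlayerHUD.
; Max-capacity events for throwables and smoke bombs only set flags.
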(event `self.ReceiveBeginPlay`
  (bind _camera (`self.Camera`))
  (bind _returnvalue (`KismetMaterialLibrary.CreateDynamicMaterialInstance` "/Game/Pawns/Player/MI_VignettePP.MI_VignettePP"))
  (bind _output_get (set `self.Vignette Material` _returnvalue))
  (bind _structout (setmembers `PostProcessSettings` :`StructRef` (`CameraComponent.PostProcessSettings` _camera) :`WeightedBlendables` (make `WeightedBlendables` (`|MakeArray` (make `WeightedBlendable` 1.0 _output_get)))))
  (set `CameraComponent.PostProcessSettings` _structout _camera)
  (`MaterialInstanceDynamic.SetScalarParameterValue` (`self.Vignette Material`) "SecondaryOpacity" 0.0))

(event `self.K2_OnStartCrouch`
  (params (HalfHeightAdjust :type "Float (single-precision)") (ScaledHalfHeightAdjust :type "Float (single-precision)"))
  (`MaterialInstanceDynamic.SetScalarParameterValue` (`self.Vignette Material`) "SecondaryOpacity" 1.0))

(event `self.K2_OnEndCrouch`
  (params (HalfHeightAdjust :type "Float (single-precision)") (ScaledHalfHeightAdjust :type "Float (single-precision)"))
  (`MaterialInstanceDynamic.SetScalarParameterValue` (`self.Vignette Material`) "SecondaryOpacity" 0.0))

(event `self.OnInventoryUpdated`
  ;[1 1 1] Update text on HUD if not max
  (bind _asplayer_hud (cast `/Game/UI/PlayerHUD` (`PlayerController.GetHUD` (`GameplayStatics.GetPlayerController` 0))))
  (bind _playerhud_ref (`/Game/UI/PlayerHUD.PlayerHUD Ref` _asplayer_hud))
  (`/Game/UI/WB_PlayerHUD.UpdateRockAmount` _playerhud_ref)
  (`/Game/UI/WB_PlayerHUD.UpdateSmokeBombAmount` _playerhud_ref))

(event `self.OnMaxThrowables`
  ;[1 1 1] If max change color
  (set `self.IsMaxThrowables` true))

(event `self.OnMaxSmokeBombs`
  ;[1 1 1] If max change color
  (set `self.IsMaxSmokeBombs` true))

(fn `UserConstructionScript`)