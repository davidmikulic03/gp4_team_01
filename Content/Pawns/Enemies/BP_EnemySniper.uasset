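; Sniper enemy Blueprint that can spin in place and kills the player with an instant-hit shot.
; Tick rotates the capsule around world Z at SpinSpeed while ShouldRotate is set.
; The Shoot event line-traces from the capsule to the supplied target position and calls Die on the hit actor if it is a PlayerCharacter.
; Targeting and the trigger for Shoot are not defined in these graphs.
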(event `self.ReceiveTick`
  (params (DeltaSeconds :type "Float (single-precision)"))
  (`parent.ReceiveTick` DeltaSeconds)
  (if (`self.ShouldRotate`)
    (`SceneComponent.K2_AddWorldRotation` (`self.CapsuleComponent`) (`KismetMathLibrary.RotatorFromAxisAndAngle` (0.0 0.0 1.0) (* DeltaSeconds (`self.Spin Speed`))) false false)))

(event `Shoot`
  (params (Target :type "Vector Structure"))
  (bind _outhit (`KismetSystemLibrary.LineTraceSingle` (`SceneComponent.K2_GetComponentLocation` (`self.CapsuleComponent`)) Target "TraceTypeQuery3"))
  (bind _asplayer_character (cast `PlayerCharacter` (`.HitActor` (`GameplayStatics.BreakHitResult` _outhit))))
  (`PlayerCharacter.Die` _asplayer_character))

(fn `UserConstructionScript`
  (`parent.UserConstructionScript`))