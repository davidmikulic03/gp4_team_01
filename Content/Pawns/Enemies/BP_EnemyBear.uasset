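; Bear enemy pawn that is immune to petrification, answering OnPetrify with only a debug print.
; On BeginPlay it caches the mesh's anim instance as ABP_Bull, the bull animation Blueprint.
; Each Tick it writes the velocity magnitude to that instance's ForwardVelocity, logic the author notes is duplicated in each enemy.
; The construction script only calls the parent's.
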(event `self.ReceiveBeginPlay`
  ;[1 1 1] this is cursed, repeated in each enemy, ew, i'm sorry
  (bind _asabp_bull (cast `/Game/Art/Enemies/Brute/ABP_Bull` (`SkeletalMeshComponent.GetAnimInstance` (`self.Mesh`))))
  (set `self.BullAnimBp` _asabp_bull))

(event `self.ReceiveTick`
  (params (DeltaSeconds :type "Float (single-precision)"))
  ;[1 1 1] this is cursed, repeated in each enemy, ew, i'm sorry
  (set `/Game/Art/Enemies/Brute/ABP_Bull.ForwardVelocity` (`KismetMathLibrary.VSize` (`self.GetVelocity`)) (`self.BullAnimBp`)))

(event `self.OnPetrify`
  (params (Player :type "PlayerCharacter Object Reference"))
  (`KismetSystemLibrary.PrintString` "Can't be petrified!"))

(fn `UserConstructionScript`
  (`parent.UserConstructionScript`))