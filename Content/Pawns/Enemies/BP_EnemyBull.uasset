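; Bull enemy that ends the game through the game mode's LoseGame when the player character enters its death overlap.
; Petrification freezes it by setting its custom time dilation to zero, then calls Unpetrify after a delay, with OnUnpetrify restoring normal time.
; Tick feeds its speed to the bull Animation Blueprint cached at BeginPlay.
; Vision-signal debug printing remains in the graph but never runs.
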(event `self.ReceiveBeginPlay`
  (bind _asabp_bull (cast `/Game/Art/Enemies/Brute/ABP_Bull` (`SkeletalMeshComponent.GetAnimInstance` (`self.Mesh`))))
  (set `self.AnimationBlueprint` _asabp_bull))

(event `self.OnUnpetrify`
  (params (Player :type "PlayerCharacter Object Reference"))
  (set `self.CustomTimeDilation` 1.0))

(event `self.OnPetrify`
  (params (Player :type "PlayerCharacter Object Reference"))
  (set `self.CustomTimeDilation` 0.0)
  (`KismetSystemLibrary.Delay` 5.0)
  (`self.Unpetrify` self self Player))

(event `self.ReceiveTick`
  (params (DeltaSeconds :type "Float (single-precision)"))
  (`|ExecutionSequence`
    (:`then_0`
      ;[1 1 1] animation bp code
      (set `/Game/Art/Enemies/Brute/ABP_Bull.ForwardVelocity` (`KismetMathLibrary.VSize` (`self.GetVelocity`)) (`self.AnimationBlueprint`)))))

(event `self.DeathOverlap.OnComponentBeginOverlap`
  (params (OverlappedComponent :type "PrimitiveComponent Object Reference") (OtherActor :type "Actor Object Reference") (OtherComp :type "PrimitiveComponent Object Reference") (OtherBodyIndex :type Integer) (bFromSweep :type Boolean) (SweepResult :type "HitResult Structure (by ref)"))
  (cast `PlayerCharacter` OtherActor)
  (bind _asmain_game_mode (cast `MainGameMode` (`GameplayStatics.GetGameMode`)))
  (`MainGameMode.LoseGame` _asmain_game_mode))

(fn `UserConstructionScript`)