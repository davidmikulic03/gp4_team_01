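; AI controller for enemy pawns that runs the BT_Popocorn behavior tree on BeginPlay.
; Fuzzy brain events for interest, signal origin and signal severity changes write TargetLocation and TargetSignalWeight to the Blackboard.
; The AI Perception update event is empty, with leftover stimulus-location and PlayerActor Blackboard writes disconnected, despite a note saying perception handles hearing.
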(event `self.ReceiveBeginPlay`
  (`self.RunBehaviorTree` "/Game/Pawns/Enemies/AI/BT_Popocorn.BT_Popocorn"))

(event `self.OnInterestChanged`
  (params (WeightedSignal :type "WeightedSignal Structure"))
  (bind (_signal _weight) (break `WeightedSignal` WeightedSignal))
  ;[1 1 1] fuzzy brain events
  (`BlackboardComponent.SetValueAsVector` (`self.Blackboard`) "TargetLocation" (`SignalFunctions.GetSignalOrigin` _signal))
  (`BlackboardComponent.SetValueAsFloat` (`self.Blackboard`) "TargetSignalWeight" _weight))

(event `self.OnSignalOriginChanged`
  (params (NewSignalOrigin :type "Vector Structure"))
  (`BlackboardComponent.SetValueAsVector` (`self.Blackboard`) "TargetLocation" NewSignalOrigin))

(event `self.OnSignalSeverityChanged`
  (params (WeightedSignal :type "WeightedSignal Structure"))
  (bind (_signal _weight) (break `WeightedSignal` WeightedSignal))
  (`BlackboardComponent.SetValueAsFloat` (`self.Blackboard`) "TargetSignalWeight" _weight)
  (`KismetSystemLibrary.PrintString` (`KismetStringLibrary.Concat_StrStr` "SIGNAL" (`KismetStringLibrary.Conv_DoubleToString` _weight)) false))

(event `self.AIPerception.OnTargetPerceptionUpdated`
  (params (Actor :type "Actor Object Reference") (Stimulus :type "AIStimulus Structure"))
  ;[1 1 1] build in perception code (only used for hearing at the moment)
)

(fn `UserConstructionScript`)