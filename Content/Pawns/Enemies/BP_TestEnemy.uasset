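; Guard enemy that shoots the player, ends the game on touch, and can be turned to stone.
; Shooting plays muzzle and sound effects, then line-traces to the target and kills any player hit.
; Petrifying applies a rock overlay, disables the death overlap and freezes it through zero custom time dilation, with a delayed unpetrify.
; Tick feeds speed to ABP_Guard; death with DoesDrop spawns gun and magnet pickups, then destroys the actor.
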(event `self.ReceiveBeginPlay`
  (bind _asabp_guard (cast `/Game/Art/Enemies/Guard/ABP_Guard` (`SkeletalMeshComponent.GetAnimInstance` (`self.Mesh`))))
  (bind _output_get (set `self.AnimationBlueprint` _asabp_guard))
  (`KismetSystemLibrary.PrintString` (`KismetSystemLibrary.GetDisplayName` _output_get)))

(event `self.OnUnpetrify`
  (params (Player :type "PlayerCharacter Object Reference"))
  (`MeshComponent.SetOverlayMaterial` (`self.Mesh`) null)
  (`PrimitiveComponent.SetCollisionEnabled` (`self.DeathOverlap`) "QueryOnly")
  (set `self.CustomTimeDilation` 1.0))

(event `self.OnPetrify`
  (params (Player :type "PlayerCharacter Object Reference"))
  (`MeshComponent.SetOverlayMaterial` (`self.Mesh`) "/Game/Art/Rocks/Rock_01/M_Rock_01.M_Rock_01")
  (`PrimitiveComponent.SetCollisionEnabled` (`self.DeathOverlap`) "NoCollision")
  (set `self.CustomTimeDilation` 0.0)
  (`KismetSystemLibrary.Delay` 5.0)
  (`self.Unpetrify` self self Player))

(event `Shoot`
  (params (Target :type "Vector Structure"))
  (bind _returnvalue (`SceneComponent.K2_GetComponentLocation` (`self.CapsuleComponent`)))
  (`NiagaraFunctionLibrary.SpawnSystemAttached` "/Game/VFX/NS_MuzzleFlash.NS_MuzzleFlash" (`self.Muzzle`) "None" (0.0 0.0 0.0) (struct) "SnapToTargetIncludingScale" true)
  (`FMODBlueprintStatics.PlayEventAtLocation` "/Game/FMOD/Events/SniperShoot.SniperShoot" (`KismetMathLibrary.Conv_VectorToTransform` _returnvalue))
  (bind _outhit (`KismetSystemLibrary.LineTraceSingle` _returnvalue Target "TraceTypeQuery3"))
  (bind _asplayer_character (cast `PlayerCharacter` (`.HitActor` (`GameplayStatics.BreakHitResult` _outhit))))
  (`PlayerCharacter.Die` _asplayer_character))

(event `self.ReceiveTick`
  (params (DeltaSeconds :type "Float (single-precision)"))
  ;[1 1 1] animation bp code
  (set `/Game/Art/Enemies/Guard/ABP_Guard.ForwardVelocity` (`KismetMathLibrary.VSize` (`self.GetVelocity`)) (`self.AnimationBlueprint`)))

(event `self.DeathOverlap.OnComponentBeginOverlap`
  (params (OverlappedComponent :type "PrimitiveComponent Object Reference") (OtherActor :type "Actor Object Reference") (OtherComp :type "PrimitiveComponent Object Reference") (OtherBodyIndex :type Integer) (bFromSweep :type Boolean) (SweepResult :type "HitResult Structure (by ref)"))
  (cast `PlayerCharacter` OtherActor)
  (bind _asmain_game_mode (cast `MainGameMode` (`GameplayStatics.GetGameMode`)))
  (`MainGameMode.LoseGame` _asmain_game_mode))

(event `self.OnDeath`
  (bind _returnvalue (- (`self.K2_GetActorLocation`) (`KismetMathLibrary.MakeVector` 0.0 0.0 (`.OutHalfHeight` (`CapsuleComponent.GetScaledCapsuleSize` (`self.CapsuleComponent`))))))
  (if (`self.Does Drop`)
    (`|SpawnActorFromClass` "/Game/Interactables/BP_GunPickup.BP_GunPickup_C" (`KismetMathLibrary.MakeTransform` (+ _returnvalue (0.0 -50.0 0.0))) "AdjustIfPossibleButAlwaysSpawn" "MultiplyWithRoot" null self)
    (`|SpawnActorFromClass` "/Game/Interactables/BP_MagnetPickup.BP_MagnetPickup_C" (`KismetMathLibrary.MakeTransform` (+ _returnvalue (0.0 50.0 0.0))) "AdjustIfPossibleButAlwaysSpawn" "MultiplyWithRoot" null self)
    (`self.K2_DestroyActor`)))

(fn `UserConstructionScript`)