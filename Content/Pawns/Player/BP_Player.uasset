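; BP_Player is the player character Blueprint, which toggles a vignette post-process effect with crouching.
; On BeginPlay it creates a dynamic instance of MI_VignettePP and sets it as the camera's post-process blendable, with secondary opacity off.
; The crouch start and end events switch the material's SecondaryOpacity parameter fully on and off, with no interpolation.
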(event `self.ReceiveBeginPlay`
  (bind _camera (`self.Camera`))
  (bind _returnvalue (`KismetMaterialLibrary.CreateDynamicMaterialInstance` "/Game/Pawns/Player/MI_VignettePP.MI_VignettePP"))
  (bind _output_get (set `self.Vignette Material` _returnvalue))
  (bind _structout (setmembers `PostProcessSettings` :`StructRef` (`CameraComponent.PostProcessSettings` _camera) :`WeightedBlendables` (make `WeightedBlendables` (`|MakeArray` (make `WeightedBlendable` 1.0 _output_get)))))
  (set `CameraComponent.PostProcessSettings` _structout _camera)
  (`MaterialInstanceDynamic.SetScalarParameterValue` (`self.Vignette Material`) "SecondaryOpacity" 0.0))

(event `self.K2_OnStartCrouch`
  (params (HalfHeightAdjust :type "Float (single-precision)") (ScaledHalfHeightAdjust :type "Float (single-precision)"))
  (`MaterialInstanceDynamic.SetScalarParameterValue` (`self.Vignette Material`) "SecondaryOpacity" 1.0))

(event `self.K2_OnEndCrouch`
  (params (HalfHeightAdjust :type "Float (single-precision)") (ScaledHalfHeightAdjust :type "Float (single-precision)"))
  (`MaterialInstanceDynamic.SetScalarParameterValue` (`self.Vignette Material`) "SecondaryOpacity" 0.0))

(fn `UserConstructionScript`)