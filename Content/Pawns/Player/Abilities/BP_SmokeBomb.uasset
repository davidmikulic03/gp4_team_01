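; BP_SmokeBomb is a player ability actor that releases an expanding smoke cloud the first time it hits something.
; On that first hit it attaches the NS_ThermalBomb Niagara effect to its Plane component, plays an attached passive smoke audio event, and sets a flag to ignore later hits.
; A timeline then scales the Plane uniformly from an initial to a final smoke size.
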(event `self.ReceiveBeginPlay`
  (set `self.HasBeenActivated` false))

(event `self.ReceiveHit`
  (params (MyComp :type "PrimitiveComponent Object Reference") (Other :type "Actor Object Reference") (OtherComp :type "PrimitiveComponent Object Reference") (bSelfMoved :type Boolean) (HitLocation :type "Vector Structure") (HitNormal :type "Vector Structure") (NormalImpulse :type "Vector Structure") (Hit :type "HitResult Structure (by ref)"))
  (if (not (`self.HasBeenActivated`))
    (`NiagaraFunctionLibrary.SpawnSystemAttached` "/Game/VFX/NS_ThermalBomb.NS_ThermalBomb" (`self.Plane`) "None" (0.0 0.0 0.0) (struct) "SnapToTargetIncludingScale")
    (`FMODBlueprintStatics.PlayEventAttached` "/Game/FMOD/Events/Smokebomb_Passive.Smokebomb_Passive" (`self.RootComponent`) "None" (0.0 0.0 0.0) "KeepRelativeOffset")
    (`self.GrowSmoke`)
    (set `self.HasBeenActivated` true)))

(event `GrowSmoke`
  (bind (_direction _growing) (`Timeline|Timeline`)
    (:`Update`
      (bind _returnvalue (`KismetMathLibrary.Lerp` (`self.InitialSmokeScale`) (`self.FinalSmokeScale`) _growing))
      (`SceneComponent.SetWorldScale3D` (`self.Plane`) (`KismetMathLibrary.MakeVector` _returnvalue _returnvalue _returnvalue)))))

(fn `UserConstructionScript`)